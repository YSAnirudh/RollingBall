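; BP_Fence is a procedural fence actor that lines up copies of a chosen mesh toward an EndPoint offset.
; The construction script divides the EndPoint's length by FenceWidth, rounds to a segment count, and adds that many static mesh components at even spacing along local X.
; Segments attach to the root Fence mesh, which is yawed toward the EndPoint, so height differences do not tilt the run.
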(fn `UserConstructionScript`
  (bind _returnvalue (`self.K2_GetActorLocation`))
  (bind _returnvalue_2 (`KismetMathLibrary.Round` (- (/ (`KismetMathLibrary.VSize` (`self.EndPoint`)) (`self.FenceWidth`)) 1.0)))
  (`StaticMeshComponent.SetStaticMesh` (`self.Fence`) (`self.SpawnMesh`))
  (if (> _returnvalue_2 0)
    (for _index (range (+ _returnvalue_2 1))
      (`|ExecutionSequence`
        (:`then_0`
          ;[1 1 1] Loop Body
          (bind _returnvalue_3 (`AddComponent|NODE_AddStaticMeshComponent-0`))
          (`SceneComponent.K2_AttachToComponent` _returnvalue_3 (`self.Fence`) "None" "KeepRelative" "KeepRelative" "KeepRelative" true)
          (`SceneComponent.K2_SetRelativeLocation` _returnvalue_3 (`KismetMathLibrary.MakeVector` (* _index (`self.FenceWidth`))) false false)
          (`StaticMeshComponent.SetStaticMesh` _returnvalue_3 (`self.SpawnMesh`)))
        (:`then_1`
          (`SceneComponent.K2_SetRelativeRotation` (`self.Fence`) (`KismetMathLibrary.MakeRotator` 0.0 0.0 (.yaw (`KismetMathLibrary.FindLookAtRotation` _returnvalue (+ _returnvalue (`self.EndPoint`))))) false false))))))